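; Game mode that spawns crevasses at random dig zones (BP_ZoneFouille) with rising difficulty.
; A BeginPlay delay loop has a random zone spawn a crevasse while fewer than three exist.
; Tick raises Difficulte with elapsed game time, shortening the delay between attempts.
; SpawnEnemy can place a BP_Ennemy at a random TargetPoint but is not called in this graph, and SpawnActorFouille is empty.
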(event EventTick
  (params (DeltaSeconds :type Float%20%28single-precision%29))
  (CallFunction|IncreaseDifficulte))

(event EventBeginPlay
  ;[1 1 1] Spawn des ennemis et crevasses
  (Utilities|FlowControl|Delay (/ (Variables|Default|GetTimer) (Math|Conversions|ToFloat(Integer) (Variables|Default|GetDifficulte))) :!label _label)
  (bind _outactors (Actor|GetAllActorsOfClass "/Game/Jeffrey/Blueprint/Fouille/BP_Crevasse.BP_Crevasse_C"))
  (if (< (Utilities|Array|LastIndex _outactors) 2)
    (bind _actorfouille (CallFunction|GetActorFouille))
    (Utilities|IsValid _actorfouille
      (:Is%20Valid
        (Default|SpawnCrevasse _actorfouille)
        (goto _label)))
    (else
      (goto _label))))

(fn ConstructionScript)

(fn GetRandomSpawnPoint
  (bind _outactors (Actor|GetAllActorsOfClass "/Script/Engine.TargetPoint"))
  (return (Utilities|Array|Get(acopy) _outactors (Math|Random|RandomIntegerinRange 0 (Utilities|Array|LastIndex _outactors)))))

(fn SpawnEnemy
  (bind _returntargetpoint (CallFunction|GetRandomSpawnPoint))
  (Utilities|IsValid _returntargetpoint
    (:Is%20Valid
      (Game|SpawnActorfromClass "/Game/Elias/Blueprint/AI/BP_Ennemy.BP_Ennemy_C" (Math|Transform|MakeTransform (Math|Vector|MakeVector (.x (.location (Transformation|GetActorTransform _returntargetpoint))) (.y (.location (Transformation|GetActorTransform _returntargetpoint))) (+ (.z (.location (Transformation|GetActorTransform _returntargetpoint))) 1.0)) (.rotation (Transformation|GetActorTransform _returntargetpoint)) (.scale (Transformation|GetActorTransform _returntargetpoint))) "Undefined" 0 0))))

(fn GetActorFouille
  (bind _outactors (Actor|GetAllActorsOfClass "/Game/Jeffrey/Blueprint/Fouille/BP_ZoneFouille.BP_ZoneFouille_C"))
  (return (Utilities|Array|Get(acopy) _outactors (Math|Random|RandomInteger (+ (Utilities|Array|LastIndex _outactors) 1)))))

(fn IncreaseDifficulte
  (Variables|Default|SetDifficulte (+ (Math|Float|Round (/ (Utilities|Time|GetGameTimeinSeconds) 1e+01)) 1)))

(fn SpawnActorFouille)