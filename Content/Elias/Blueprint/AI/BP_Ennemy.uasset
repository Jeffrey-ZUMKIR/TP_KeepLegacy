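; Enemy character with one of two random flipbook looks that seeks out and attacks crevasses, and that the player damages by clicking it.
; MoveToZone sends it by AI MoveTo to a random BP_Crevasse, retrying until it claims an available one.
; It then loops attack animations and damage until that crevasse is gone, then moves on.
; Clicks reduce life and update the HUD widget; death frees the crevasse and destroys the enemy.
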(event Custom|onAttackCrevasse
  (bind _crevasse (Variables|Default|Getcrevasse))
  (Development|PrintString "collision")
  ;[1 1 1] attack crevasse
  (if (Variables|Default|GetisAttacking)
    (if (== (Variables|Default|GetenemyType) 2)
      (bind _returnvalue (Sprite|SetFlipbook (Variables|Default|GetspriteAnimation) "/Game/Elias/animations/discovery/enemy2_Discovery.enemy2_Discovery"))
      (Utilities|FlowControl|Delay (Math|Conversions|ToFloat(Boolean) _returnvalue))
      (else
        (bind _returnvalue_2 (Sprite|SetFlipbook (Variables|Default|GetspriteAnimation) "/Game/Elias/animations/discovery/enemy_Discovery.enemy_Discovery"))
        (Utilities|FlowControl|Delay (Math|Conversions|ToFloat(Boolean) _returnvalue_2))))
    (if (== (Variables|Default|GetenemyType) 2) :!label _label
      (bind _returnvalue_3 (Sprite|SetFlipbook (Variables|Default|GetspriteAnimation) "/Game/Elias/animations/attack/enemy2_attack1.enemy2_attack1"))
      (Utilities|FlowControl|Delay (Math|Conversions|ToFloat(Boolean) _returnvalue_3))
      (Sprite|SetFlipbook (Variables|Default|GetspriteAnimation) "/Game/Elias/animations/attack/enemy2_attack2.enemy2_attack2")
      (else
        (bind _returnvalue_4 (Sprite|SetFlipbook (Variables|Default|GetspriteAnimation) "/Game/Elias/animations/attack/enemy_attack1.enemy_attack1"))
        (Utilities|FlowControl|Delay (Math|Conversions|ToFloat(Boolean) _returnvalue_4))
        (Sprite|SetFlipbook (Variables|Default|GetspriteAnimation) "/Game/Elias/animations/attack/enemy_attack2.enemy_attack2")))
    (Utilities|IsValid _crevasse
      (:Is%20Valid
        (Game|Damage|ApplyDamage _crevasse 1.0 0 self)
        (Utilities|FlowControl|Delay 1.0)
        (Utilities|IsValid (Variables|Default|Getcrevasse)
          (:Is%20Valid
            (if (== (Variables|Default|GetenemyType) 2)
              (Sprite|SetFlipbook (Variables|Default|GetspriteAnimation) "/Game/Elias/animations/attack/enemy2_attack1.enemy2_attack1")
              (goto _label)
              (else
                (Sprite|SetFlipbook (Variables|Default|GetspriteAnimation) "/Game/Elias/animations/attack/enemy_attack1.enemy_attack1")
                (goto _label))))
          (:Is%20Not%20Valid
            (if (== (Variables|Default|GetenemyType) 2)
              (Sprite|SetFlipbook (Variables|Default|GetspriteAnimation) "/Game/Elias/animations/attack/enemy2_attack1.enemy2_attack1")
              (else
                (Sprite|SetFlipbook (Variables|Default|GetspriteAnimation) "/Game/Elias/animations/attack/enemy_attack1.enemy_attack1")))
            (Variables|Default|SetisAttacking false)
            (if (== (Variables|Default|GetenemyType) 2)
              (Sprite|SetFlipbook (Variables|Default|GetspriteAnimation) "/Game/Elias/animations/walkAnimation/enemy2_Walk.enemy2_Walk")
              (else
                (Sprite|SetFlipbook (Variables|Default|GetspriteAnimation) "/Game/Elias/animations/walkAnimation/enemy_walk.enemy_walk")))
            (Utilities|MovetoZone))))
      (:Is%20Not%20Valid
        (Variables|Default|SetisAttacking false)))))

(event EventBeginPlay
  (bind _output_get (Variables|Default|SetenemyType (Math|Random|RandomIntegerinRange 1 2)))
  (if (== _output_get 2)
    (Sprite|SetFlipbook (Variables|Default|GetspriteAnimation) "/Game/Elias/animations/idle/enemy2_idle.enemy2_idle")
    (else
      (Sprite|SetFlipbook (Variables|Default|GetspriteAnimation) "/Game/Elias/animations/idle/enemy_idle.enemy_idle")))
  ;[1 1 1] Initialisation barre de vie ennemi
  (bind _ashud_ennemy (Utilities|Casting|CastToHUD_Ennemy (UserInterface|GetUserWidgetObject (Variables|Default|GetWidget))))
  (bind _output_get_2 (Variables|Default|SetwidgetHUD_Enemy _ashud_ennemy))
  (CallFunction|MajWidgetLife _output_get_2)
  ;[1 1 1] déplacement des ennemies vers les zones
  (if (and (not (CallFunction|IsDead)) (not false))
    (Utilities|FlowControl|Delay 2.0)
    (Utilities|MovetoZone)))

(event EventTick
  (params (DeltaSeconds :type Float%20%28single-precision%29))
  ;[1 1 1] on oblige les instances ennemies à rester droit au cours de leurs déplacements
  (Transformation|SetActorRotation "0,-180.000000, 0")
  (if (<= (.x (Transformation|GetActorLocation)) 0.0)
    (Transformation|SetRelativeRotation (Variables|Default|GetspriteAnimation) "180.000000,-90.000000,-90.000000" false false)
    (else
      (Transformation|SetRelativeRotation (Variables|Default|GetspriteAnimation) "0.000000,-90.000000,-90.000000" false false))))

(event MouseInput|EventActorOnClicked
  (params (ButtonPressed :type Key%20Structure :default "None"))
  (CallFunction|ApplyDamages)
  ;[1 1 1] degats ennemis
  (CallFunction|MajWidgetLife (Variables|Default|GetwidgetHUD_Enemy))
  (if (== (Variables|Default|GetenemyType) 2)
    (bind _returnvalue (Sprite|SetFlipbook (Variables|Default|GetspriteAnimation) "/Game/Elias/animations/degats/enemy2_Degats.enemy2_Degats"))
    (Utilities|FlowControl|Delay (Math|Conversions|ToFloat(Boolean) _returnvalue))
    (else
      (bind _returnvalue_2 (Sprite|SetFlipbook (Variables|Default|GetspriteAnimation) "/Game/Elias/animations/degats/enemy_Degats.enemy_Degats"))
      (Utilities|FlowControl|Delay (Math|Conversions|ToFloat(Boolean) _returnvalue_2))))
  (if (CallFunction|IsDead)
    (Variables|/Game/Jeffrey/Blueprint/Fouille/BP_Crevasse.BP_Crevasse_C|SetIs%20Available (Variables|Default|Getcrevasse) true)
    (Pawn|Components|CharacterMovement|DisableMovement (Variables|Character|GetCharacterMovement self))
    (bind _returnvalue_3 (Sprite|SetFlipbook (Variables|Default|GetspriteAnimation) "/Game/Elias/animations/death/death.death"))
    (Utilities|FlowControl|Delay (Math|Conversions|ToFloat(Boolean) _returnvalue_3))
    (Actor|DestroyActor)))

(fn ConstructionScript)

(fn IsDead
  (bind _output_get (Variables|Default|SetisDeadEnemy (<= (Variables|Default|Getnb_Life) 0.0)))
  (return _output_get))

(fn MajWidgetLife
  (params (widgetHUD_Enemy :type HUD%20Ennemy%20Object%20Reference))
  (Variables|/Game/Elias/UI/HUD_Ennemy.HUD_Ennemy_C|Setnb_lifeEnnemy widgetHUD_Enemy (Variables|Default|Getnb_Life)))

(fn ApplyDamages
  (Variables|Default|Setnb_Life (- (Variables|Default|Getnb_Life) 25.0)))