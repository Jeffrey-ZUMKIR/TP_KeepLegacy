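; BP_Connaissance is an actor that shows the player's knowledge score through a widget and ends the level when it reaches the maximum.
; Every tick it reads Score and MaxScore from BP_GameInstance and pushes the ratio and values to the WDG_Connaissance progress display in its widget component.
; Once Score reaches MaxScore, it opens the Menu level.
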(event EventBeginPlay)

(event Collision|EventActorBeginOverlap
  (params (OtherActor :type Actor%20Object%20Reference)))

(event EventTick
  (params (DeltaSeconds :type Float%20%28single-precision%29))
  (bind _asbp_game_instance (Utilities|Casting|CastToBP_GameInstance (Game|GetGameInstance)))
  (bind _aswdg_connaissance (Utilities|Casting|CastToWDG_Connaissance (UserInterface|GetWidget (Variables|Default|GetWidget))))
  (Default|SetProgress _aswdg_connaissance (/ (Variables|/Game/Jeffrey/Blueprint/GameInstance/BP_GameInstance.BP_GameInstance_C|GetScore _asbp_game_instance) (Variables|/Game/Jeffrey/Blueprint/GameInstance/BP_GameInstance.BP_GameInstance_C|GetMaxScore _asbp_game_instance)))
  (Default|SetProgressText _aswdg_connaissance (Variables|/Game/Jeffrey/Blueprint/GameInstance/BP_GameInstance.BP_GameInstance_C|GetScore _asbp_game_instance) (Variables|/Game/Jeffrey/Blueprint/GameInstance/BP_GameInstance.BP_GameInstance_C|GetMaxScore _asbp_game_instance))
  (if (>= (Variables|/Game/Jeffrey/Blueprint/GameInstance/BP_GameInstance.BP_GameInstance_C|GetScore _asbp_game_instance) (Variables|/Game/Jeffrey/Blueprint/GameInstance/BP_GameInstance.BP_GameInstance_C|GetMaxScore _asbp_game_instance))
    (Game|OpenLevel(byName) "Menu")))

(fn ConstructionScript)