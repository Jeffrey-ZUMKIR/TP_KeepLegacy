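; BP_GameModeJeff is a game mode that periodically spawns BP_Crevasse actors inside the level's dig zones.
; From BeginPlay, an endless delay loop picks a random BP_ZoneFouille and spawns a crevasse slightly above it, owned by that zone.
; Helper functions apply random X and Y offsets around the zone's location, with a wider spread on Y.
; Each new crevasse receives a random rarity (Rarete) from three levels.
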(event EventBeginPlay
  (Utilities|FlowControl|Delay (Variables|Default|GetTimer) :!label _label)
  (bind _actor_fouille (CallFunction|GetActorFouille))
  (bind _returnvalue (Game|SpawnActorfromClass "/Game/Jeffrey/Blueprint/Fouille/BP_Crevasse.BP_Crevasse_C" (Math|Transform|MakeTransform (Math|Vector|MakeVector (CallFunction|GetRandomX (.x (.location (Transformation|GetActorTransform _actor_fouille)))) (CallFunction|GetRandomY (.y (.location (Transformation|GetActorTransform _actor_fouille)))) (+ (.z (.location (Transformation|GetActorTransform _actor_fouille))) 1.0)) (.rotation (Transformation|GetActorTransform _actor_fouille)) "1,1,1") "Undefined" _actor_fouille 0))
  (Variables|/Game/Jeffrey/Blueprint/Fouille/BP_Crevasse.BP_Crevasse_C|SetRarete _returnvalue (Math|Random|RandomInteger 3))
  (goto _label))

(event EventTick
  (params (DeltaSeconds :type Float%20%28single-precision%29)))

(fn ConstructionScript)

(fn GetActorFouille
  (bind _outactors (Actor|GetAllActorsOfClass "/Game/Jeffrey/Blueprint/Fouille/BP_ZoneFouille.BP_ZoneFouille_C"))
  (return (Utilities|Array|Get(acopy) _outactors (Math|Random|RandomInteger (+ (Utilities|Array|LastIndex _outactors) 1)))))

(fn GetRandomX
  (params (A :type Float%20%28single-precision%29))
  (return (Math|Conversions|ToFloat(Integer) (+ (- (Math|Random|RandomInteger 400) 200) (Math|Float|Truncate A)))))

(fn GetRandomY
  (params (A :type Float%20%28single-precision%29))
  (return (Math|Conversions|ToFloat(Integer) (+ (- (Math|Random|RandomInteger 800) 400) (Math|Float|Truncate A)))))