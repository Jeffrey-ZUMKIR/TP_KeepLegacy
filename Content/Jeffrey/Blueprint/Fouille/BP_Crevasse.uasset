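; BP_Crevasse is a clickable crevasse actor that is worn down by damage until it is destroyed.
; Its Onspawn event rolls one of three rarity tiers, weighted toward the most common, with rarer tiers getting more health.
; Each click applies one damage to itself through AnyDamage, which destroys it at zero health.
; Spawn and non-lethal hits push current and maximum health to its WDG_Health widget component.
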(event Custom|On%20spawn
  (switch int (Math|Random|RandomInteger 9)
    (:0
      (bind _output_get (Variables|Default|SetMaxHealth 2 :!label _label))
      (Variables|Default|SetHealth _output_get)
      (Variables|Default|SetRarete 1))
    (:1
      (goto _label))
    (:2
      (goto _label))
    (:3
      (goto _label))
    (:4
      (goto _label))
    (:5
      (goto _label))
    (:6
      (bind _output_get_2 (Variables|Default|SetMaxHealth 5 :!label _label_2))
      (Variables|Default|SetHealth _output_get_2)
      (Variables|Default|SetRarete 2))
    (:7
      (goto _label_2))
    (:8
      (bind _output_get_3 (Variables|Default|SetMaxHealth 10))
      (Variables|Default|SetHealth _output_get_3)
      (Variables|Default|SetRarete 3)))
  (bind _aswdg_health (Utilities|Casting|CastToWDG_Health (UserInterface|GetUserWidgetObject (Variables|Default|GetWDG_Health))))
  (Variables|/Game/Jeffrey/Blueprint/Fouille/WDG_Health.WDG_Health_C|SetHealth _aswdg_health (Math|Conversions|ToFloat(Integer) (Variables|Default|GetHealth)))
  (Variables|/Game/Jeffrey/Blueprint/Fouille/WDG_Health.WDG_Health_C|SetMaxHealth _aswdg_health (Math|Conversions|ToFloat(Integer) (Variables|Default|GetMaxHealth))))

(event EventBeginPlay)

(event Collision|EventActorBeginOverlap
  (params (OtherActor :type Actor%20Object%20Reference)))

(event EventTick
  (params (DeltaSeconds :type Float%20%28single-precision%29)))

(event Game|Damage|EventAnyDamage
  (params (Damage :type Float%20%28single-precision%29) (DamageType :type Damage%20Type%20Object%20Reference) (InstigatedBy :type Controller%20Object%20Reference) (DamageCauser :type Actor%20Object%20Reference))
  (bind _output_get (Variables|Default|SetHealth (- (Variables|Default|GetHealth) (Math|Float|Truncate Damage))))
  (if (<= _output_get 0)
    (Actor|DestroyActor)
    (else
      (bind _aswdg_health (Utilities|Casting|CastToWDG_Health (UserInterface|GetUserWidgetObject (Variables|Default|GetWDG_Health))))
      (Variables|/Game/Jeffrey/Blueprint/Fouille/WDG_Health.WDG_Health_C|SetHealth _aswdg_health (Math|Conversions|ToFloat(Integer) (Variables|Default|GetHealth)))
      (Variables|/Game/Jeffrey/Blueprint/Fouille/WDG_Health.WDG_Health_C|SetMaxHealth _aswdg_health (Math|Conversions|ToFloat(Integer) (Variables|Default|GetMaxHealth))))))

(event MouseInput|EventActorOnClicked
  (params (ButtonPressed :type Key%20Structure :default "None"))
  (Game|Damage|ApplyDamage self 1.0 0 0))

(fn ConstructionScript)