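; BP_ZoneFouille is a dig zone actor that spawns BP_Crevasse actors at random spots within its area.
; When Spawn_Crevasse is called and the Spawn flag is set, it places a crevasse slightly above its own height, attaches it to itself and calls OnSpawn on it.
; GetRandomX and GetRandomY offset the zone's location within a world-axis rectangle that is twice as long in Y as in X.
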(event Custom|Spawn_Crevasse
  (bind _returnvalue (Transformation|GetActorTransform))
  (if (Variables|Default|GetSpawn)
    (bind _returnvalue_2 (Game|SpawnActorfromClass "/Game/Jeffrey/Blueprint/Fouille/BP_Crevasse.BP_Crevasse_C" (Math|Transform|MakeTransform (Math|Vector|MakeVector (CallFunction|GetRandomX (.x (.location _returnvalue))) (CallFunction|GetRandomY (.y (.location _returnvalue))) (+ (.z (.location _returnvalue)) 1.0)) (.rotation _returnvalue) "1,1,1") "Undefined" 0 0))
    (Transformation|AttachActorToActor _returnvalue_2 self "None" "KeepWorld" "KeepRelative" "KeepWorld" true)
    (Default|OnSpawn _returnvalue_2)))

(event EventBeginPlay)

(event Collision|EventActorBeginOverlap
  (params (OtherActor :type Actor%20Object%20Reference)))

(event EventTick
  (params (DeltaSeconds :type Float%20%28single-precision%29)))

(fn ConstructionScript)

(fn GetRandomX
  (params (A :type Float%20%28single-precision%29))
  (return (Math|Conversions|ToFloat(Integer) (+ (- (Math|Random|RandomInteger 300) 150) (Math|Float|Truncate A)))))

(fn GetRandomY
  (params (A :type Float%20%28single-precision%29))
  (return (Math|Conversions|ToFloat(Integer) (+ (- (Math|Random|RandomInteger 600) 300) (Math|Float|Truncate A)))))